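; Lane actor that shows one of two merged grass meshes, dark or light, picked at random on BeginPlay.
; LaneRandomizer repeats the same random mesh pick as a callable function, though BeginPlay uses its own inline copy.
; GetArrow returns the world transform of the Arrow component.
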(event `self.ReceiveBeginPlay`
  (`StaticMeshComponent.SetStaticMesh` (`self.StaticMesh`) (select `int` (`KismetMathLibrary.RandomIntegerInRange` 0 1) :`0` "/Game/Meshes/SM_MERGED_SM_MERGED_darkgrass_2.SM_MERGED_SM_MERGED_darkgrass_2" :`1` "/Game/Meshes/SM_MERGED_SM_MERGED_litegrass_6.SM_MERGED_SM_MERGED_litegrass_6" :!type "StaticMesh Object Reference")))

(fn `GetArrow`
  (returns (lanetransform :type "Transform Structure"))
  (return (`SceneComponent.K2_GetComponentToWorld` (`self.Arrow`))))

(fn `LaneRandomizer`
  (`StaticMeshComponent.SetStaticMesh` (`self.StaticMesh`) (select `int` (`KismetMathLibrary.RandomIntegerInRange` 0 1) :`0` "/Game/Meshes/SM_MERGED_SM_MERGED_darkgrass_2.SM_MERGED_SM_MERGED_darkgrass_2" :`1` "/Game/Meshes/SM_MERGED_SM_MERGED_litegrass_6.SM_MERGED_SM_MERGED_litegrass_6" :!type "StaticMesh Object Reference")))

(fn `UserConstructionScript`)