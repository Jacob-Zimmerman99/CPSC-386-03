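; BP_PLAYER is a player character that jumps automatically while its movement keys are held.
; Forward and right axis inputs add movement relative to control-rotation yaw.
; W, A, S and D actions share one JumpTest flag, set on press and cleared on any release.
; Tick calls Jump while the flag is set, with StopJumping after a one-second Delay, and calls StopJumping whenever it is clear.
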(event `InputAxis|Moveforward`
  (params (AxisValue :type "Float (single-precision)"))
  (bind (_returnvalue_roll _returnvalue_pitch _returnvalue_yaw) (`KismetMathLibrary.BreakRotator` (`self.GetControlRotation`)))
  (`self.AddMovementInput` (`KismetMathLibrary.GetForwardVector` (`KismetMathLibrary.MakeRotator` 0.0 0.0 _returnvalue_yaw)) AxisValue))

(event `InputAction|W`
  (params (Key :type "Key Structure"))
  (:`Pressed`
    (set `self.jump_test` true))
  (:`Released`
    (set `self.jump_test` false)))

(event `InputAction|D`
  (params (Key :type "Key Structure"))
  (:`Pressed`
    (set `self.jump_test` true))
  (:`Released`
    (set `self.jump_test` false)))

(event `InputAxis|MoveRight`
  (params (AxisValue :type "Float (single-precision)"))
  (bind (_returnvalue_roll _returnvalue_pitch _returnvalue_yaw) (`KismetMathLibrary.BreakRotator` (`self.GetControlRotation`)))
  (`self.AddMovementInput` (`KismetMathLibrary.GetRightVector` (`KismetMathLibrary.MakeRotator` 0.0 0.0 _returnvalue_yaw)) AxisValue))

(event `InputAction|A`
  (params (Key :type "Key Structure"))
  (:`Pressed`
    (set `self.jump_test` true))
  (:`Released`
    (set `self.jump_test` false)))

(event `InputAction|S`
  (params (Key :type "Key Structure"))
  (:`Pressed`
    (set `self.jump_test` true))
  (:`Released`
    (set `self.jump_test` false)))

(event `self.ReceiveTick`
  (params (DeltaSeconds :type "Float (single-precision)"))
  (if (`self.jump_test`)
    (`self.Jump`)
    (`KismetSystemLibrary.Delay` 1.0)
    (`self.StopJumping`)
    (else
      (`self.StopJumping`))))

(fn `UserConstructionScript`)